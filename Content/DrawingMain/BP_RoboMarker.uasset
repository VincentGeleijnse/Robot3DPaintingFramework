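; Robot marker pen actor that draws on a canvas while following a G-code path.
; While the pen is enabled, each tick runs a short line trace along its up vector to detect the canvas.
; Hits become collision UVs for continuous line drawing, colored from the imported G-code palette by the path follower's current color index.
; When the trace finds no canvas, it ends the stroke.
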(event EventBeginPlay
  (Variables|Default|Setpathfollow (Actor|GetComponentbyClass "/Script/RobotArm.FollowGCodePathRobot")))

(event EventTick
  (params (DeltaSeconds :type Float%20%28single-precision%29))
  (bind _returnvalue (Transformation|GetActorUpVector))
  (bind _returnvalue_2 (Transformation|GetActorLocation))
  (if (Variables|Default|GetEnable%20Pen)
    (bind _outhit (Collision|LineTraceByChannel (+ _returnvalue_2 (* _returnvalue 7.0)) (+ _returnvalue_2 (* _returnvalue 8.0)) "TraceTypeQuery1" true 0 "None"))
    (bind _asmy_main_canvas_bp (Utilities|Casting|CastToMyMainCanvasBP (.HitActor (Collision|BreakHitResult _outhit)))
      (:then
        (Variables|/Game/DrawingMain/Blueprints/MyMainCanvasBP.MyMainCanvasBP_C|SetDraw%20Color _asmy_main_canvas_bp (Utilities|Array|Get(acopy) (Variables|/Script/RobotArm.ImportGCode|GetcolorArr (Variables|Default|GetImportGCode)) (Variables|/Script/RobotArm.FollowGCodePathRobot|Getcolor (Variables|Default|Getpathfollow))))
        (Default|DrawContinousLine _asmy_main_canvas_bp (.UV (Class|GameplayStatics|FindCollisionUV _outhit))))
      (:CastFailed
        (Default|EndDraw (Variables|Default|GetCanvas))))))

(event Collision|EventActorBeginOverlap
  (params (OtherActor :type Actor%20Object%20Reference)))

(fn ConstructionScript)