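; Drawing canvas actor that a pen paints on through a render target shown on the Canvas mesh by a dynamic material.
; BeginPlay creates and clears the target, and if wrapping is enabled, copies the mesh geometry and canvas transform to the SplinePathResolver's FollowGCodePathRobot component.
; DrawContinousLine turns UV-style hit locations into connected segments, scaling thickness by canvas size, with EndDraw restarting the stroke.
; Image loading and hit-driven drawing in the event graph are disconnected.
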(event Custom|End%20Draw
  ;[1 1 1] Start or finish draw
  (Variables|Default|SetDrawEnable false)
  (Variables|Default|SetPenStayOnSurface true))

(event Custom|Start%20Draw
  ;[1 1 1] Start or finish draw
  (Variables|Default|SetDrawEnable true))

(event EventBeginPlay
  (bind _splinepathresolver (Variables|Default|GetSplinePathResolver))
  (bind _returnvalue (Actor|GetComponentbyClass _splinepathresolver "/Script/RobotArm.FollowGCodePathRobot"))
  (CallFunction|InitializeRenderTarget)
  (if (Variables|/Script/RobotArm.FollowGCodePathRobot|GetWrapping _returnvalue)
    (bind (_vertices _triangles _normals _uvs) (Class|KismetProceduralMeshLibrary|GetSectionfromStaticMesh (Variables|/Script/Engine.StaticMeshComponent|GetStaticMesh (Variables|Default|GetCanvas))))
    (Variables|/Script/RobotArm.FollowGCodePathRobot|SetVertices _returnvalue _vertices)
    (Variables|/Script/RobotArm.FollowGCodePathRobot|SetTriangles _returnvalue _triangles)
    (Variables|/Script/RobotArm.FollowGCodePathRobot|SetNormals _returnvalue _normals)
    (Variables|/Script/RobotArm.FollowGCodePathRobot|SetUVs _returnvalue _uvs)
    (Variables|/Script/RobotArm.FollowGCodePathRobot|SetcanvasPos _returnvalue (Transformation|GetActorLocation))
    (Variables|/Script/RobotArm.FollowGCodePathRobot|SetcanvasScale _returnvalue (Transformation|GetActorScale3D))
    (Development|PrintString (Utilities|String|Append (Utilities|String|ToString(Integer) (Utilities|Array|Length _triangles)) " triangles and" (Utilities|String|ToString(Integer) (Utilities|Array|Length _vertices)) " verts"))))

(event Collision|EventActorBeginOverlap
  (params (OtherActor :type Actor%20Object%20Reference)))

(event EventTick
  (params (DeltaSeconds :type Float%20%28single-precision%29)))

(fn ConstructionScript)

(fn InitializeRenderTarget
  (bind _board_resolution (Variables|Default|GetBoard%20Resolution))
  (bind (_x _y) (Math|Vector2D|BreakVector2D _board_resolution))
  (Rendering|CreateRenderTarget2D (Math|Float|Truncate _x) (Math|Float|Truncate _y) "RTF_RGBA16f")
  (Rendering|ClearRenderTarget2D (Variables|Default|GetCanvas) (Variables|Default|GetRT) (Variables|Default|GetStartColor))
  (bind _returnvalue (Rendering|Material|CreateDynamicMaterialInstance "/Game/DrawingMain/Materials/Components/M_RenderTarget.M_RenderTarget" "None" "None" :!class /Script/Engine.KismetMaterialLibrary))
  (Rendering|Material|SetTextureParameterValue _returnvalue "RT" (Variables|Default|GetRT))
  (bind _output_get (Variables|Default|SetMATERIAL _returnvalue))
  (Rendering|Material|SetMaterial (Variables|Default|GetCanvas) 0 _output_get))

(fn DrawContinousLine
  (params (HitLocation :type Vector%202D%20Structure))
  (Variables|Default|SetIn%20Progress true)
  (if (Variables|Default|GetPenStayOnSurface)
    ;[1 1 1] Save first dot. (to draw line with 2 coords)
    (Variables|Default|SetFirstDot (* HitLocation (Variables|Default|GetBoard%20Resolution)))
    (Variables|Default|SetPenStayOnSurface false)
    (Variables|Default|SetIn%20Progress false)
    (else
      (bind (_canvas _size _context) (Rendering|BeginDrawCanvastoRenderTarget (Variables|Default|GetRT)))
      (Class|Canvas|DrawLine _canvas (Variables|Default|GetFirstDot) (* _size HitLocation) (* (Variables|Default|GetSize) (/ 1.0 (Math|Vector|GetMaxElement (Transformation|GetWorldScale (Variables|Default|GetCanvas))))) (Variables|Default|GetDraw%20Color))
      (Rendering|EndDrawCanvastoRenderTarget _context)
      (Variables|Default|SetIn%20Progress false)
      (Variables|Default|SetFirstDot (* _size HitLocation)))))