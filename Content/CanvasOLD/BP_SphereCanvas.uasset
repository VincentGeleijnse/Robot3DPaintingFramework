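; Paintable canvas actor that draws marker strokes into a render target, with a configurable canvas mesh.
; On BeginPlay it creates a dynamic M_Marker instance, clears two render targets and derives trace offsets from the mesh bounds.
; SurfacePositionNormal queries surface info each tick using numpad-adjusted Y/Z values.
; DrawOnCanvas sets the marker's location and color, then draws it to RT_Canvas.
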(event Custom|Draw%20On%20Canvas
  (params (DrawLocation :type Vector%202D%20Structure) (Color :type Linear%20Color%20Structure))
  (bind _marker_mi (Variables|Default|GetMarker_MI))
  (Rendering|Material|SetVectorParameterValue _marker_mi "DrawLocation" (Math|Conversions|ToLinearColor(Vector) (Math|Conversions|ToVector(Vector2D) DrawLocation)) :!class /Script/Engine.MaterialInstanceDynamic)
  (Rendering|Material|SetVectorParameterValue _marker_mi "BrushColor" Color :!class /Script/Engine.MaterialInstanceDynamic)
  (Rendering|DrawMaterialtoRenderTarget "/Game/CanvasOLD/RT_Canvas.RT_Canvas" _marker_mi))

(event EventBeginPlay
  (bind _surfacepositionnormal (Variables|Default|GetSurfacePositionNormal))
  (bind _canvas (Variables|Default|GetCanvas))
  (bind (_min _max) (Components|StaticMesh|GetLocalBounds _canvas))
  (bind _returnvalue (Rendering|Material|CreateDynamicMaterialInstance "/Game/CanvasOLD/M_Marker.M_Marker" "None" "None" :!class /Script/Engine.KismetMaterialLibrary))
  (Variables|Default|SetMarker_MI _returnvalue)
  (Rendering|ClearRenderTarget2D "/Game/CanvasOLD/RT_Canvas.RT_Canvas")
  (Rendering|ClearRenderTarget2D "/Game/CanvasOLD/RT_Canvas1.RT_Canvas1")
  (Variables|/Game/CanvasOLD/SurfacePositionNormal.SurfacePositionNormal_C|SetTraceOffsetmin _surfacepositionnormal (/ _max 2.0))
  (Variables|/Game/CanvasOLD/SurfacePositionNormal.SurfacePositionNormal_C|SetTraceOffsetmax _surfacepositionnormal (/ _min 2.0))
  (Input|EnableInput (Game|GetPlayerController 0)))

(event Collision|EventActorBeginOverlap
  (params (OtherActor :type Actor%20Object%20Reference)))

(event EventTick
  (params (DeltaSeconds :type Float%20%28single-precision%29))
  (Default|GetSurfaceInfo (Variables|Default|GetSurfacePositionNormal) (Variables|Default|GetY) (Variables|Default|GetZ)))

(event Input|KeyboardEvents|NumPadFour
  (params (Key :type Key%20Structure))
  (:Pressed
    (Math|Float|DecrementFloat (Variables|Default|GetY))))

(event Input|KeyboardEvents|NumPadNine
  (params (Key :type Key%20Structure))
  (:Pressed
    (Variables|Default|SetOtherColor (not (Variables|Default|GetOtherColor)))))

(event Input|KeyboardEvents|NumPadEight
  (params (Key :type Key%20Structure))
  (:Pressed
    (Math|Float|IncrementFloat (Variables|Default|GetZ))))

(event Input|KeyboardEvents|NumPadTwo
  (params (Key :type Key%20Structure))
  (:Pressed
    (Math|Float|DecrementFloat (Variables|Default|GetZ))))

(event Input|KeyboardEvents|NumPadSix
  (params (Key :type Key%20Structure))
  (:Pressed
    (Math|Float|IncrementFloat (Variables|Default|GetY))))

(fn ConstructionScript
  (Components|StaticMesh|SetStaticMesh (Variables|Default|GetCanvas) (Variables|Default|GetCanvas%20Mesh)))